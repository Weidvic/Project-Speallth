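; Player character Blueprint for an owl with world-axis movement, mouse aiming of the head and projectile firing.
; Each tick the head mesh yaws toward the cursor hit point with an offset, keeping the body's pitch and roll.
; W, A, S and D presses play timelines that lerp the body toward fixed facings, independent of the movement axes.
; Fire spawns an Arrow at FirePoint and launches it along its right vector.
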(event `InputAxis|MoveUp`
  (params (AxisValue :type "Float (single-precision)"))
  ;[1 1 1] Movement
  (`self.AddMovementInput` (1.0 0.0 0.0) AxisValue))

(event `InputAxis|MoveRight`
  (params (AxisValue :type "Float (single-precision)"))
  ;[1 1 1] Movement
  (`self.AddMovementInput` (0.0 1.0 0.0) AxisValue))

(event `self.ReceiveTick`
  (params (DeltaSeconds :type "Float (single-precision)"))
  (bind (_returnvalue_roll _returnvalue_pitch) (`KismetMathLibrary.BreakRotator` (`SceneComponent.K2_GetComponentRotation` (`self.Owl_Body`))))
  (bind (_returnvalue_roll_2 _returnvalue_pitch_2 _returnvalue_yaw) (`KismetMathLibrary.BreakRotator` (`KismetMathLibrary.FindLookAtRotation` (`SceneComponent.K2_GetComponentLocation` (`self.Owl_Head`)) (`.Location` (`GameplayStatics.BreakHitResult` (`PlayerController.GetHitResultUnderCursorByChannel` (`GameplayStatics.GetPlayerController` 0) "TraceTypeQuery1" true))))))
  ;[1 1 1] Turn head to look at mouse - Head mesh rotation is probably off lol
  (`SceneComponent.K2_SetWorldRotation` (`self.Owl_Head`) (`KismetMathLibrary.MakeRotator` _returnvalue_roll _returnvalue_pitch (+ _returnvalue_yaw -90.0)) false false))

(event `Key|S`
  (params (Key :type "Key Structure"))
  (bind _owl_body (`self.Owl_Body`))
  ;[1 1 1] Rotating body to look at direction of movement - NEEDS TWEAKING
  (:`Pressed`
    (`Timeline|Timeline_1` :`NewTime` 0.2 :!via `PlayFromStart`
      (:`Update`
        (`SceneComponent.K2_SetWorldRotation` _owl_body (`KismetMathLibrary.RLerp` (`SceneComponent.K2_GetComponentRotation` _owl_body) (struct :`Yaw` 90.0) 0.2 true) false false)))))

(event `Key|W`
  (params (Key :type "Key Structure"))
  (bind _owl_body (`self.Owl_Body`))
  ;[1 1 1] Rotating body to look at direction of movement - NEEDS TWEAKING
  (:`Pressed`
    (`Timeline|Timeline_2` :`NewTime` 0.2 :!via `PlayFromStart`
      (:`Update`
        (`SceneComponent.K2_SetWorldRotation` _owl_body (`KismetMathLibrary.RLerp` (`SceneComponent.K2_GetComponentRotation` _owl_body) (struct :`Yaw` -90.0) 0.2 true) false false)))))

(event `Key|A`
  (params (Key :type "Key Structure"))
  (bind _owl_body (`self.Owl_Body`))
  ;[1 1 1] Rotating body to look at direction of movement - NEEDS TWEAKING
  (:`Pressed`
    (`Timeline|RotationTimeline` :`NewTime` 0.2 :!via `PlayFromStart`
      (:`Update`
        (`SceneComponent.K2_SetWorldRotation` _owl_body (`KismetMathLibrary.RLerp` (`SceneComponent.K2_GetComponentRotation` _owl_body) (struct :`Yaw` 180.0) 0.2 true) false false)))))

(event `InputAction|Fire`
  (params (Key :type "Key Structure"))
  (bind _firepoint (`self.FirePoint`))
  ;[1 1 1] Firing Base Projectile
  (:`Pressed`
    (bind _returnvalue (`|SpawnActorFromClass` "/Game/ProjectSpellth/Placeholders/Arrow/Arrow.Arrow_C" (`KismetMathLibrary.MakeTransform` (`SceneComponent.K2_GetComponentLocation` _firepoint) (`SceneComponent.K2_GetComponentRotation` _firepoint)) "Undefined" "OverrideRootScale" null null))
    (bind _output_get (set `self.Projectile` _returnvalue))
    (set `MovementComponent.Velocity` (* (`SceneComponent.GetRightVector` (`Actor.RootComponent` (`self.Projectile`))) 800.0) (`/Game/ProjectSpellth/Placeholders/Arrow/Arrow.ProjectileMovement` _output_get))))

(event `Key|D`
  (params (Key :type "Key Structure"))
  (bind _owl_body (`self.Owl_Body`))
  ;[1 1 1] Rotating body to look at direction of movement - NEEDS TWEAKING
  (:`Pressed`
    (`Timeline|Timeline_0` :`NewTime` 0.2 :!via `PlayFromStart`
      (:`Update`
        (`SceneComponent.K2_SetWorldRotation` _owl_body (`KismetMathLibrary.RLerp` (`SceneComponent.K2_GetComponentRotation` _owl_body) (struct) 0.2 true) false false)))))

(fn `UserConstructionScript`)