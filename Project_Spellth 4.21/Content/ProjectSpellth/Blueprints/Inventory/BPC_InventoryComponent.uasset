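; BPC_InventoryComponent is an inventory component that stores slot structures and displays them in a spell window.
; On BeginPlay it creates WB_SpellWindow bound to itself, anchors it bottom-center on the player controller's HUD canvas, and sizes the slot array.
; AddToInventory calls CreateStack, which writes content into the first slot matching an empty structure.
; It always returns true, with no check for a full inventory or merging of existing stacks.
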(event `self.ReceiveBeginPlay`
  (bind _returnvalue (`|CreateWidget` "/Game/ProjectSpellth/Blueprints/Inventory/SpellUI/WB_SpellWindow.WB_SpellWindow_C" null self))
  (set `self.InventoryWindow` _returnvalue)
  (bind _asbp_player_controller (cast `/Game/ProjectSpellth/PlayerCharacter/BP_PlayerController` (`GameplayStatics.GetPlayerController` 0)))
  (bind _returnvalue_2 (`CanvasPanel.AddChildToCanvas` (`/Game/ProjectSpellth/Blueprints/Inventory/SpellUI/WB_Hud.HudCanvas` (`/Game/ProjectSpellth/PlayerCharacter/BP_PlayerController.Hud Widget` _asbp_player_controller)) (`self.InventoryWindow`)))
  (`CanvasPanelSlot.SetAutoSize` _returnvalue_2 true)
  (`CanvasPanelSlot.SetAlignment` _returnvalue_2 (0.5 0.5))
  (`CanvasPanelSlot.SetAnchors` _returnvalue_2 (make `Anchors` (0.5 1.0) (0.5 1.0)))
  (`CanvasPanelSlot.SetPosition` _returnvalue_2 (`self.Position`))
  (`self.PrepareInventory`))

(fn `AddToInventory`
  (params (ContentToAdd :type "/Game/ProjectSpellth/Blueprints/Inventory/SlotStructure Structure"))
  (returns (`Success?` :type Boolean))
  (`self.CreateStack` (`local.ContentToAdd`))
  (return true))

(fn `CreateStack`
  (params (ContentToAdd :type "/Game/ProjectSpellth/Blueprints/Inventory/SlotStructure Structure"))
  (bind _inventory (`self.Inventory`))
  ;[1 1 1] Find empty space and fill it
  (`KismetArrayLibrary.Array_Set` _inventory (`KismetArrayLibrary.Array_Find` _inventory (make `/Game/ProjectSpellth/Blueprints/Inventory/SlotStructure` (struct :`Name` "NSLOCTEXT(\"[1D54F4C7480FEBE20ECB9880B471F2BE]\", \"EA223D6B442F11C5220715AC178FAA0B\", \"None\")" :`Description` "NSLOCTEXT(\"[1D54F4C7480FEBE20ECB9880B471F2BE]\", \"A0C30513484B38B5CF11F09847FBCA25\", \"None\")"))) ContentToAdd))

(fn `PrepareInventory`
  (`KismetArrayLibrary.Array_Resize` (`self.Inventory`) (`self.NumberOfSlots`)))